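; Mortar actor Blueprint that acts as an aiming weapon emplacement with an on-screen health bar.
; On BeginPlay it initialises its TankAiming component with the Barrel and Turret parts.
; It then casts its Widget component's user widget to HealthBar and passes itself as the TankRef, reusing the tank health bar widget.
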(event `self.ReceiveBeginPlay`
  (`TankAimingComponent.Initialise` (`self.TankAiming`) (`self.Barrel`) (`self.Turret`))
  (`self.Set Health Bar Widget`))

(fn `Set Health Bar Widget`
  (bind _ashealth_bar (cast `/Game/Blueprints/HealthBar` (`WidgetComponent.GetUserWidgetObject` (`self.Widget`))))
  (set `/Game/Blueprints/HealthBar.TankRef` self _ashealth_bar))

(fn `UserConstructionScript`)