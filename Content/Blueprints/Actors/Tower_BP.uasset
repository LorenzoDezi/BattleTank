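; Tower actor that displays a health bar through a 3D widget component.
; On BeginPlay it registers itself as the HealthBar widget's associated actor.
; Each Tick it rotates the widget to face opposite the player Tank_BP camera's forward vector, keeping the bar billboarded to the view.
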(event `self.ReceiveBeginPlay`
  (bind _ashealth_bar (cast `/Game/Blueprints/UI/HealthBar` (`WidgetComponent.GetUserWidgetObject` (`self.Widget`))))
  (set `/Game/Blueprints/UI/HealthBar.WidgetAssociatedActor` self _ashealth_bar))

(event `self.ReceiveTick`
  (params (DeltaSeconds :type "Float (single-precision)"))
  ;[1 1 1] Set 3D Widget rotation properly
  (bind _astank_bp (cast `/Game/Blueprints/Actors/Tank_BP` (`GameplayStatics.GetPlayerPawn` 0)))
  (`SceneComponent.K2_SetWorldRotation` (`self.Widget`) (`KismetMathLibrary.Conv_VectorToRotator` (`KismetMathLibrary.NegateVector` (`SceneComponent.GetForwardVector` (`/Game/Blueprints/Actors/Tank_BP.Camera` _astank_bp)))) false false))

(fn `UserConstructionScript`)