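; Player-controlled tank pawn Blueprint that wires input to its movement and aiming components.
; BeginPlay hands the barrel and turret to TankAiming and the left and right propulsors to TankMovement.
; Keyboard and other axes drive forward and turn intents, with turning reduced to full left or right by sign.
; Aim axes rotate the spring arm and azimuth gimbal, while Fire and Boost call the components, boosting along the last forward input.
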(event `self.ReceiveBeginPlay`
  (`TankAimingComponent.Initialise` (`self.TankAiming`) (`self.Barrel`) (`self.Turret`))
  (`TankMovementComponent.Initialise` (`self.TankMovement`) (`self.LeftPropulsor`) (`self.RightPropulsor`)))

(event `InputAxis|Forward_Movement_Keyboard`
  (params (AxisValue :type "Float (single-precision)"))
  ;[1 1 1] Movement Binding
  (set `self.BoostDirection` AxisValue)
  (`TankMovementComponent.IntendMoveForward` (`self.TankMovement`) AxisValue))

(event `InputAxis|AimElevation`
  (params (AxisValue :type "Float (single-precision)"))
  ;[1 1 1] Aim/Fire Binding
  (`SceneComponent.K2_AddLocalRotation` (`self.SpringArm`) (`KismetMathLibrary.MakeRotator` 0.0 AxisValue) false false))

(event `InputAxis|Forward_Movement`
  (params (AxisValue :type "Float (single-precision)"))
  ;[1 1 1] Movement Binding
  (set `self.BoostDirection` AxisValue)
  (`TankMovementComponent.IntendMoveForward` (`self.TankMovement`) AxisValue))

(event `InputAxis|AimAzimuth`
  (params (AxisValue :type "Float (single-precision)"))
  ;[1 1 1] Aim/Fire Binding
  (`SceneComponent.K2_AddLocalRotation` (`self.AzimuthGimbal`) (`KismetMathLibrary.MakeRotator` 0.0 0.0 AxisValue) false false))

(event `InputAction|Boost`
  (params (Key :type "Key Structure"))
  ;[1 1 1] Movement Binding
  (:`Pressed`
    (`TankMovementComponent.Boost` (`self.TankMovement`) (`self.BoostDirection`))))

(event `InputAction|Fire`
  (params (Key :type "Key Structure"))
  ;[1 1 1] Aim/Fire Binding
  (:`Pressed`
    (`TankAimingComponent.Fire` (`self.TankAiming`))))

(event `InputAxis|Rotate_Movement_Keyboard`
  (params (AxisValue :type "Float (single-precision)"))
  (bind _tankmovement (`self.TankMovement`))
  ;[1 1 1] Movement Binding
  (`/Engine/EditorBlueprintResources/StandardMacros.CompareFloat` AxisValue
    (:`>`
      (`TankMovementComponent.IntendTurnRight` _tankmovement 1.0))
    (:`<`
      (`TankMovementComponent.IntendTurnLeft` _tankmovement 1.0))))

(event `InputAxis|Rotate_Movement`
  (params (AxisValue :type "Float (single-precision)"))
  (bind _tankmovement (`self.TankMovement`))
  ;[1 1 1] Movement Binding
  (`/Engine/EditorBlueprintResources/StandardMacros.CompareFloat` AxisValue
    (:`>`
      (`TankMovementComponent.IntendTurnRight` _tankmovement 1.0))
    (:`<`
      (`TankMovementComponent.IntendTurnLeft` _tankmovement 1.0))))

(fn `UserConstructionScript`)