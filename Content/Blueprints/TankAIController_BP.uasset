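; AI controller for tank pawns that runs the tank behavior tree and blackboard on BeginPlay.
; AI perception writes sensed actors lacking the "Enemy" tag to the player blackboard key and clears that key when such an actor is lost.
; An EndedSetup event tells the controlled Machine_BP pawn to set up its health bar widget.
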(event `self.EndedSetup`
  ;[1 1 1] Set User UI Widget
  (bind _asmachine_bp (cast `/Game/Blueprints/Machine_BP` (`self.K2_GetPawn`)))
  (`/Game/Blueprints/Machine_BP.SetHealthBarWidget` _asmachine_bp))

(event `self.ReceiveBeginPlay`
  ;[1 1 1] Set User UI Widget
  (bind _blackboardcomponent (`self.UseBlackboard` "/Game/Blueprints/TankBlackboard.TankBlackboard"))
  (set `self.BlackboardComponent` _blackboardcomponent)
  (`self.RunBehaviorTree` "/Game/Blueprints/TankBehaviour.TankBehaviour"))

(event `self.AIPerception.OnTargetPerceptionUpdated`
  (params (Actor :type "Actor Object Reference") (Stimulus :type "AIStimulus Structure"))
  (bind _blackboardcomponent (`self.BlackboardComponent`))
  (bind _tankplayerkey (`self.TankPlayerKey`))
  ;[1 1 1] OnAIPerceptionUpdate
  (if (`self.ActorHasTag` Actor "Enemy")
    _
    (elif (`.bSuccessfullySensed` (break `AIStimulus` Stimulus))
      (`BlackboardComponent.SetValueAsObject` _blackboardcomponent _tankplayerkey Actor)
      (else
        (`BlackboardComponent.ClearValue` _blackboardcomponent _tankplayerkey)))))

(fn `UserConstructionScript`)